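; BP_EnemyMage is a mage enemy that travels a fixed path of six waypoints and can be killed.
; Tick slides the Mesh, not the actor, at constant speed toward the target selected by CurrentPoint, without sweep.
; Near a point it increments the index, yaws 90 degrees either way and calls Andar to reinitialise animation.
; PerdeVida removes one health point and triggers MorteInimigo, which destroys the actor when none remain.
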(event Custom|MorteInimigo
  ;[1 1 1] Morte do Inimigo
  (Actor|DestroyActor))

(event Custom|PerdeVida
  ;[1 1 1] Tirando a vida do Inimigo
  (bind _result (Math|Integer|DecrementInt (Variables|Default|GetVidaInimigo))
    (:%20%20
      (Variables|Default|SetVidaInimigo _result)
      (if (< (Variables|Default|GetVidaInimigo) 1)
        (CallFunction|MorteInimigo)))))

(event Custom|Andar
  ;[0.15 0.15 0.15 0.5] Animação Inimigo
  (Components|Animation|SetAnimationMode (Variables|Character|GetMesh) (Class|SkeletalMeshComponent|GetAnimationMode (Variables|Character|GetMesh)) true))

(event EventTick
  (params (DeltaSeconds :type Float%20%28single-precision%29))
  (bind _mesh (Variables|Character|GetMesh))
  (bind _mesh_2 (Variables|Character|GetMesh))
  (bind _returnvalue (Transformation|GetWorldLocation _mesh))
  ;[1 1 1] Movimentação
  (Transformation|SetWorldLocation (Variables|Character|GetMesh) (Math|Interpolation|VInterptoConstant _returnvalue (Transformation|GetActorLocation (Variables|Default|GetTargetAtual)) DeltaSeconds 5e+01) false false)
  (switch int (Variables|Default|GetCurrentPoint)
    (:1
      (Variables|Default|SetTargetAtual (Variables|Default|GetPonto01)))
    (:2
      (Variables|Default|SetTargetAtual (Variables|Default|GetPonto02)))
    (:3
      (Variables|Default|SetTargetAtual (Variables|Default|GetPonto03)))
    (:4
      (Variables|Default|SetTargetAtual (Variables|Default|GetPonto04)))
    (:5
      (Variables|Default|SetTargetAtual (Variables|Default|GetPonto05)))
    (:6
      (Variables|Default|SetTargetAtual (Variables|Default|GetPonto06))))
  (if (< (Math|Vector|Distance(Vector) _returnvalue (Transformation|GetActorLocation (Variables|Default|GetTargetAtual))) 5e+01)
    (bind _result (Math|Integer|IncrementInt (Variables|Default|GetCurrentPoint))
      (:%20%20
        (Variables|Default|SetCurrentPoint _result)
        (if (or (== (Variables|Default|GetTargetAtual) (Variables|Default|GetPonto03)) (== (Variables|Default|GetTargetAtual) (Variables|Default|GetPonto04)))
          (Transformation|AddWorldRotation _mesh_2 "0.000000,90.000000,0.000000" false false)
          (CallFunction|Andar)
          (else
            (Transformation|AddWorldRotation _mesh_2 "0.000000,-90.000000,0.000000" false false)
            (CallFunction|Andar)))))))

(fn ConstructionScript)