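; Enemy spawner actor that creates a set number of BP_Enemy instances at its own transform.
; The SpawnEnemy event calls NewFunction, which always spawns regardless of collision and passes six Ponto point variables to each enemy.
; It increments a spawned counter and calls itself again after a one-second delay until the target count is reached.
; The file only defines the event; nothing in it triggers the first spawn.
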(event Custom|Spawn%20Enemy
  (CallFunction|NewFunction (Transformation|GetActorTransform) (Variables|Default|GetPonto01) (Variables|Default|GetPonto02) (Variables|Default|GetPonto03) (Variables|Default|GetPonto04) (Variables|Default|GetPonto05) (Variables|Default|GetPonto06))
  (Variables|Default|SetSpawnedEnimies (+ (Variables|Default|GetSpawnedEnimies) 1))
  (if (> (Variables|Default|GetEnimiesToSpawner) (Variables|Default|GetSpawnedEnimies))
    (Utilities|FlowControl|Delay 1.0)
    (CallFunction|SpawnEnemy)))

(fn ConstructionScript)

(fn NewFunction
  (params (SpawnTransform :type Transform) (Ponto01 :type Actor%20Object%20Reference) (Ponto02 :type Actor%20Object%20Reference) (Ponto03 :type Actor%20Object%20Reference) (Ponto04 :type Actor%20Object%20Reference) (Ponto05 :type Actor%20Object%20Reference) (Ponto06 :type Actor%20Object%20Reference))
  (Game|SpawnActorfromClass "/Game/MyGame/Inimigos/BP_Enemy.BP_Enemy_C" SpawnTransform "AlwaysSpawn" "MultiplyWithRoot" 0 Ponto01 Ponto02 Ponto03 Ponto04 Ponto05 Ponto06 0))